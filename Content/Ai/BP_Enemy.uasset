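; Base AI enemy character with stats, lock-on health widgets, data-table attack selection, taunts and sprint-ram reactions.
; Timer-driven hand sphere traces deal damage to non-enemies with hitstop and impact effects.
; Player damage lowers stats and triggers overridable reactions: randomized montage, knockback and stun reported to the AI controller alongside movement and attack state.
; Death plays a montage, drops rune currency, clears target lock, dissolves the mesh and notifies its spawner.
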(event OnComponentBeginOverlap(CapsuleComponent)
  (params (OverlappedComponent :type Primitive%20Component%20Object%20Reference) (OtherActor :type Actor%20Object%20Reference) (OtherComp :type Primitive%20Component%20Object%20Reference) (OtherBodyIndex :type Integer) (bFromSweep :type Boolean) (SweepResult :type Hit%20Result%20Structure%20%28by%20ref%29))
  (bind _self self)
  (bind _thirdpersonref (Variables|Default|GetThirdPersonRef))
  (Class|KismetSystemLibrary|IsObjectOfSoftClass OtherActor "/Game/Characters/ThirdPerson/Blueprints/BP_ThirdPersonCharacter.BP_ThirdPersonCharacter_C"
    (:True
      (if (and (>= (Math|Vector|VectorLength (Transformation|GetVelocity OtherActor)) 1.25e+03) (Variables|/Game/Characters/ThirdPerson/Blueprints/BP_ThirdPersonCharacter.BP_ThirdPersonCharacter_C|GetSprinting? (Variables|Default|GetThirdPersonRef)))
        (Game|Damage|ApplyDamage _self 0.01 (Game|GetInstigatorController _thirdpersonref) _thirdpersonref "/Game/Blueprints/DamageTypes/DT_PotImpact.DT_PotImpact_C")
        (Niagara|SpawnSystematLocation "/Game/FX/VFX/Vefects/Anime_VFX/Shared/Skills/NS_GenericImpact.NS_GenericImpact" (Transformation|GetActorLocation _self) "0, 0, 0" "1.000000,1.000000,1.000000" true true "AutoRelease" false)
        (Variables|Actor|SetbCanBeDamaged false)
        (Utilities|Time|SetTimerbyFunctionName 0 "DamageTimer" 0.5)
        (Default|CameraShake (Variables|Default|GetThirdPersonRef))))))

(event Custom|SmoothSetRotation
  (params (TargetRotation :type Rotator))
  ;[0.15 0.15 0.15 0.5] Start timeline to smoothly lerp rotation
  (bind _0_1 (Timeline|Timeline PlayFromStart)
    (:Update
      (Transformation|SetActorRotation (Math|Rotator|Lerp(Rotator) (Transformation|GetActorRotation) TargetRotation _0_1 true)))))

(event Custom|Damage%20Trace
  (bind _self self)
  ;[0.15 0.15 0.15 0.5] Sword Trace
  (bind (_tracestart _traceend _tracesize) (CallFunction|MatchDamageTraceData (stale EventBeginSwordTrace DamageTraceName)))
  (bind (_outhit _returnvalue) (Collision|SphereTraceForObjects _tracestart _traceend _tracesize (Utilities|Array|MakeArray "ObjectTypeQuery3") false (Variables|Default|GetAlreadyDamagedActors) "None"))
  (if _returnvalue
    (Class|KismetSystemLibrary|IsObjectOfSoftClass (.HitActor (Collision|BreakHitResult _outhit)) "/Game/Ai/BP_Enemy.BP_Enemy_C"
      (:False
        (Game|Damage|ApplyDamage (.HitActor (Collision|BreakHitResult _outhit)) (stale EventBeginSwordTrace Damage) (Pawn|GetController _self) _self (stale EventBeginSwordTrace DamageType))
        (Utilities|Array|Add (Variables|Default|GetAlreadyDamagedActors) (.HitActor (Collision|BreakHitResult _outhit)))
        (CallFunction|StartHitstop (Variables|Default|GetHitstopDuration))
        (Niagara|SpawnSystematLocation "/Game/FX/VFX/Vefects/Anime_VFX/Shared/Skills/NS_GenericImpact.NS_GenericImpact" (- (.ImpactPoint (Collision|BreakHitResult _outhit)) (* (.ImpactNormal (Collision|BreakHitResult _outhit)) 6e+01)) "0, 0, 0" "1.000000,1.000000,1.000000" true true "AutoRelease" false)))))

(event Custom|StartHitstop
  (params (Duration :type Float%20%28double-precision%29))
  (bind _mesh (Variables|Character|GetMesh))
  ;[0.15 0.15 0.15 0.5] Hitstop
  (Variables|/Script/Engine.SkeletalMeshComponent|SetbPauseAnims _mesh true)
  (Utilities|FlowControl|RetriggerableDelay Duration)
  (Variables|/Script/Engine.SkeletalMeshComponent|SetbPauseAnims _mesh false))

(event Custom|StartStun
  (params (Duration :type Float%20%28double-precision%29))
  (bind _aicontroller (Variables|Default|GetAIController))
  ;[0.15 0.15 0.15 0.5] AI Stun
  (Default|UpdateIsStunned _aicontroller true)
  (Utilities|FlowControl|RetriggerableDelay Duration)
  (Default|UpdateIsStunned _aicontroller false))

(event Custom|EnableWidget
  ;[0.15 0.15 0.15 0.5] TargetLock
  (Rendering|SetVisibility (Variables|Default|GetTargetLockWidget) true false)
  (bind _asenemy_health (Utilities|Casting|CastToEnemy_Health (UserInterface|GetWidget (Variables|Default|GetHealthWidget))))
  (Variables|/Game/UI/Enemy_Health.Enemy_Health_C|SetLockedOn? _asenemy_health true)
  (Default|DisplayMe _asenemy_health))

(event Custom|DisableWidget
  ;[0.15 0.15 0.15 0.5] TargetLock
  (Rendering|SetVisibility (Variables|Default|GetTargetLockWidget) false false)
  (bind _asenemy_health (Utilities|Casting|CastToEnemy_Health (UserInterface|GetWidget (Variables|Default|GetHealthWidget))))
  (Variables|/Game/UI/Enemy_Health.Enemy_Health_C|SetLockedOn? _asenemy_health false)
  (Default|HideMe _asenemy_health))

(event Custom|Drop%20Coins/Runes
  ;[0.15 0.15 0.15 0.5] Enemy drop coins/Runes
  (for _index (range 0 (- (Variables|Default|GetCurrencyOnDrop) 1))
    (bind _randomlocation (Class|NavigationSystemV1|GetRandomLocationinNavigableRadius (.location (Transformation|GetActorTransform)) 3e+02 0 0))
    (bind _returnvalue (Game|SpawnActorfromClass "/Game/Blueprints/Collectables/BP_RuneCurrency01.BP_RuneCurrency01_C" (Math|Transform|MakeTransform _randomlocation "0, 0, 0" "1.000000,1.000000,1.000000") "Undefined" "MultiplyWithRoot" 0 0))
    (Default|ChooseMesh _returnvalue)
    (Default|Moveto _returnvalue (.location (Transformation|GetActorTransform)) _randomlocation)))

(event EventOnMovementModeChanged
  (params (PrevMovementMode :type EMovementMode%20Enum :default "MOVE_None") (NewMovementMode :type EMovementMode%20Enum :default "MOVE_None") (PrevCustomMode :type Byte :default 0) (NewCustomMode :type Byte :default 0))
  ;[0.15 0.15 0.15 0.5] Report new MovementMode changes to AI Behaviour Tree
  (bind _aicontroller (Variables|Default|GetAIController)
    (:then
      (Default|UpdateMovementMode _aicontroller PrevMovementMode NewMovementMode))
    (:else)))

(event EventBeginSwordTrace
  (params (Damage :type Float%20%28double-precision%29) (DamageType :type Damage%20Type%20Class%20Reference) (DamageTraceName :type Name :default "None"))
  ;[0.15 0.15 0.15 0.5] Sword Trace
  (Utilities|Array|Clear (Variables|Default|GetAlreadyDamagedActors))
  (bind _returnvalue (Utilities|Time|SetTimerbyEvent (delegate Custom|Damage%20Trace) 0.01 true)))

(event EventEndSwordTrace
  ;[0.15 0.15 0.15 0.5] Sword Trace
  (if (Utilities|Time|IsValidTimerHandle (stale EventBeginSwordTrace _returnvalue))
    (Utilities|Time|ClearandInvalidateTimerbyHandle (stale EventBeginSwordTrace _returnvalue))))

(event EventBeginPlay
  (bind _maxspeedvariance (Variables|Default|GetMaxSpeedVariance))
  (bind _charactermovement (Variables|Character|GetCharacterMovement))
  ;[0.15 0.15 0.15 0.5] Initialize Stats
  ;[0.15 0.15 0.15 0.5] AddViewmodel
  (bind _asenemy_health (Utilities|Casting|CastToEnemy_Health (UserInterface|GetWidget (Variables|Default|GetHealthWidget)) :!label _label))
  (Utilities|IsValid (Variables|/Game/UI/Enemy_Health.Enemy_Health_C|GetViewModelStatsEnemy _asenemy_health)
    (:Is%20Valid
      (Default|SetViewModel (Variables|Default|GetBPC_Stats) (Variables|/Game/UI/Enemy_Health.Enemy_Health_C|GetViewModelStatsEnemy _asenemy_health))
      (bind _asbp_ai_enemy (Utilities|Casting|CastToBP_AI_Enemy (AI|GetAIController self)))
      (Variables|Default|SetAIController _asbp_ai_enemy)
      (bind _returnvalue (Rendering|Material|CreateDynamicMaterialInstance (Rendering|Material|GetMaterial (Variables|Character|GetMesh) 0) "None" "None" :!class /Script/Engine.KismetMaterialLibrary))
      (Rendering|Material|SetMaterial (Variables|Character|GetMesh) 0 _returnvalue)
      (Variables|Default|SetMaterialInstance _returnvalue)
      ;[0.15 0.15 0.15 0.5] Apply random speed variance to enemies so they move less predictably in unison
      (Variables|/Script/Engine.CharacterMovementComponent|SetMaxWalkSpeed _charactermovement (+ (Class|MovementComponent|GetMaxSpeed _charactermovement) (Math|Random|RandomFloatinRange (* _maxspeedvariance -1.0) _maxspeedvariance)))
      ;[0.15 0.15 0.15 0.5] Set Third Person Ref
      (bind _outactors (Actor|GetAllActorsOfClass "/Game/Characters/ThirdPerson/Blueprints/BP_ThirdPersonCharacter.BP_ThirdPersonCharacter_C"))
      (Variables|Default|SetThirdPersonRef (Utilities|Array|Get(acopy) _outactors)))
    (:Is%20Not%20Valid
      (Utilities|FlowControl|Delay 0.2)
      (goto _label))))

(event Game|Damage|EventAnyDamage
  (params (Damage :type Float%20%28single-precision%29) (DamageType :type Damage%20Type%20Object%20Reference) (InstigatedBy :type Controller%20Object%20Reference) (DamageCauser :type Actor%20Object%20Reference))
  ;[0.15 0.15 0.15 0.5] Take Damage
  (if (Class|Controller|IsPlayerController InstigatedBy)
    (Default|IncreaseValue (Variables|Default|GetBPC_Stats) "NewEnumerator0" (* Damage -1.0))
    (CallFunction|OnDamageReaction Damage DamageType DamageCauser)
    (Variables|/Script/Engine.CharacterMovementComponent|SetGravityScale (Variables|Character|GetCharacterMovement) 1.5)))

(event EventDie
  (bind _capsulecomponent (Variables|Collision|GetCapsuleComponent))
  (bind _mesh (Variables|Character|GetMesh))
  ;[0.15 0.15 0.15 0.5] Death
  (Niagara|SpawnSystematLocation "/Game/FX/VFX/Basic_VFX/Niagara/NS_GoblinDeath.NS_GoblinDeath" (Transformation|GetActorLocation self))
  (Utilities|FlowControl|Delay 0.15) ; Bandaid fix to allow enough time for hit reaction animations to blend nicely
  (Variables|Default|SetIsDead? true)
  (Components|Movement|StopMovementImmediately (Variables|Character|GetCharacterMovement))
  (Default|Die (Variables|Default|GetAIController))
  (Animation|Montage|PlayMontage _mesh (Variables|Montages|GetDeathMontage)
    (:then
      (CallFunction|DropCoins/Runes)
      (Collision|SetCollisionResponsetoChannel _capsulecomponent "ECC_Pawn" "ECR_Ignore")
      (Collision|SetCollisionObjectType _capsulecomponent "ECC_PhysicsBody")
      (|ClearTargetLockonplayeriflockedbythem)
      (Rendering|SetVisibility (Variables|Default|GetTargetLockWidget) false false)
      (Utilities|FlowControl|Delay 2.5)
      (bind _dissolveparam (Timeline|DissolveTimeline PlayFromStart)
        (:Update
          (Rendering|Material|SetScalarParameterValue (Variables|Default|GetMaterialInstance) "Dissolve" _dissolveparam :!class /Script/Engine.MaterialInstanceDynamic))
        (:Finished
          (Rendering|SetVisibility (Variables|Default|GetHealthWidget) false false)
          (bind _spawnerreference (Variables|Default|GetSpawnerReference)
            (:then
              (Default|DecrementTotalEnemies _spawnerreference))
            (:else)))))
    (:OnBlendOut
      (Variables|/Script/Engine.SkeletalMeshComponent|SetbPauseAnims _mesh true) ; Hacky way to stop the death montage at last frame long enough for enemy to vanish, you could add a proper IsDead check to enemy ABP instead
    )))

(event EventSelectAttack
  (bind _attackstochoosefrom (Variables|Default|GetAttacksToChooseFrom))
  ;[0.15 0.15 0.15 0.5] Select Anim To Play
  (Utilities|Array|Clear (Variables|Default|GetAttacksToChooseFrom))
  (bind _outrownames (DataTable|GetDataTableRowNames (Variables|Default|GetAttackList)))
  (for _array_element _outrownames
    (bind _returnvalue (Utilities|GetDataTableRow (Variables|Default|GetAttackList) _array_element)
      (:then
        (if (Utilities|Enum|Equal(Enum) (.AttackType (Utilities|Struct|BreakF_EnemyAttacks _returnvalue)) "NewEnumerator0")
          (Utilities|Array|Add (Variables|Default|GetAttacksToChooseFrom) _array_element)))))
  (bind _returnvalue_2 (Utilities|GetDataTableRow (Variables|Default|GetAttackList) (Utilities|Array|Get(acopy) _attackstochoosefrom (Math|Random|RandomInteger (Utilities|Array|Length _attackstochoosefrom))))
    (:then
      (Variables|Default|SetAnimToPlay (.Animation (Utilities|Struct|BreakF_EnemyAttacks _returnvalue_2)))
      (Default|SetRadius (Variables|Default|GetAIController) (.Radius (Utilities|Struct|BreakF_EnemyAttacks _returnvalue_2))))))

(fn ConstructionScript)

(fn OnDamageReaction
  (params (Damage :type Float%20%28double-precision%29) (DamageType :type Damage%20Type%20Object%20Reference) (DamageCauser :type Actor%20Object%20Reference))
  (bind _returnvalue (Transformation|GetActorLocation DamageCauser))
  (bind _asdt_melee (Utilities|Casting|CastToDT_Melee DamageType)) ; WIll add in support for other damage outside melee when needed
  (if (.FoundMontage? (|FindRandomizedHitReactMontage (Variables|Montages|GetHitReactionMontages) (Variables|/Game/Blueprints/DamageTypes/DT_Melee.DT_Melee_C|GetHitReactionType _asdt_melee)))
    (bind _returnvalue_2 (Animation|PlayAnimMontage (.Montage (|FindRandomizedHitReactMontage (Variables|Montages|GetHitReactionMontages) (Variables|/Game/Blueprints/DamageTypes/DT_Melee.DT_Melee_C|GetHitReactionType _asdt_melee))) 1.0 "None")))
  (CallFunction|StartStun _returnvalue_2)
  (CallFunction|ApplyKnockbackfromSource (|ApplyRandomizedVariance (Variables|/Game/Blueprints/DamageTypes/DT_Melee.DT_Melee_C|GetAttackKnockback _asdt_melee) (Variables|/Game/Blueprints/DamageTypes/DT_Melee.DT_Melee_C|GetRandomizedKnockbackVariance _asdt_melee)) _returnvalue)
  (Audio|SpawnSoundatLocation (Variables|/Game/Blueprints/DamageTypes/DT_Melee.DT_Melee_C|GetSound _asdt_melee) _returnvalue "0, 0, 0" 1.0 1.0 0.0 0 0))

(fn ApplyKnockbackfromSource
  (params (KnockbackForce :type Vector) (SourceLocation :type Vector))
  (bind _returnvalue (Transformation|GetActorLocation))
  (bind _returnvalue_2 (Math|Rotator|FindLookatRotation SourceLocation _returnvalue))
  (bind _returnvalue_3 (Math|Rotator|MakeRotator 0.0 0.0 (.yaw _returnvalue_2)))
  (Components|Movement|StopMovementImmediately (Variables|Character|GetCharacterMovement))
  (Character|LaunchCharacter (Math|Vector|RotateVector KnockbackForce _returnvalue_3) true true)
  (CallFunction|SmoothSetRotation (Utilities|GetOppositeDirection _returnvalue_3)))

(fn DamageTimer
  (Variables|Actor|SetbCanBeDamaged true))

(fn BasicAttack
  (Default|IsAttacking? (Variables|Default|GetAIController) true)
  (bind _returnvalue (Animation|PlayAnimMontage (Variables|Default|GetAnimToPlay) 1.0 "None"))
  (return _returnvalue))

(fn Launch)

(fn MatchDamageTraceData
  (params (DamageTraceName :type Name :default "None"))
  (switch name DamageTraceName
    (:Default
      (Utilities|Debugging|RaiseScriptError "Invalid Damage Trace Provided!")
      (return "0, 0, 0" "0, 0, 0" 0.0))
    (:LeftHand
      (return (Transformation|GetWorldLocation (Variables|Default|GetLTraceStart)) (Transformation|GetWorldLocation (Variables|Default|GetLTraceEnd)) 4e+01))
    (:RightHand
      (return (Transformation|GetWorldLocation (Variables|Default|GetRTraceStart)) (Transformation|GetWorldLocation (Variables|Default|GetRTraceEnd)) 4e+01))))

(fn Taunt
  (bind _tauntmontages (Variables|Montages|GetTauntMontages))
  (bind _returnvalue (Animation|PlayAnimMontage (Utilities|Set|GetItemByIndex _tauntmontages (Math|Random|RandomInteger (Utilities|Set|Length _tauntmontages))) 1.0 "None"))
  (return _returnvalue))