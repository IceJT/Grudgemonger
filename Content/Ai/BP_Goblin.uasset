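; Goblin character Blueprint that provides a forward leap attack and the trace shapes for its damage checks.
; Launch throws it along its capsule's forward vector with added lift, temporarily loosening gravity, braking, floor-angle and step limits and ignoring Pawn collision, then sets normal values after a delay.
; MatchDamageTraceData maps a trace name (left hand, right hand or ball) to scene-component locations and a radius, raising a script error for unknown names.
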(event EventBeginPlay
  (|CallParentFunction) ; This node is disabled and will not be called.\nDrag off pins to build functionality.
)

(event Collision|EventActorBeginOverlap
  (params (OtherActor :type Actor%20Object%20Reference)))

(event EventTick
  (params (DeltaSeconds :type Float%20%28single-precision%29)))

(event EventLaunch
  (bind _charactermovement (Variables|Character|GetCharacterMovement))
  (bind _charactermovement_2 (Variables|Character|GetCharacterMovement))
  (Character|LaunchCharacter (+ (* (Math|Vector|GetForwardVector (Variables|Default|GetCapsuleComponent)) (Variables|Default|GetLaunchVelocity)) "0.000000,0.000000,250.000000") false false)
  (Variables|/Script/Engine.CharacterMovementComponent|SetBrakingFrictionFactor _charactermovement_2 0.2)
  (Variables|/Script/Engine.CharacterMovementComponent|SetGravityScale _charactermovement_2 0.3)
  (Pawn|Components|CharacterMovement|SetWalkableFloorAngle _charactermovement_2 9e+01)
  (Variables|/Script/Engine.CharacterMovementComponent|SetMaxStepHeight _charactermovement_2 1e+02)
  (Collision|SetCollisionResponsetoChannel (Variables|Default|GetCapsuleComponent) "ECC_Pawn" "ECR_Ignore")
  (Utilities|FlowControl|Delay 1.5)
  (Collision|SetCollisionResponsetoChannel (Variables|Default|GetCapsuleComponent) "ECC_Pawn" "ECR_Block")
  (Variables|/Script/Engine.CharacterMovementComponent|SetBrakingFrictionFactor _charactermovement 2.0)
  (Variables|/Script/Engine.CharacterMovementComponent|SetGravityScale _charactermovement 1.5)
  (Pawn|Components|CharacterMovement|SetWalkableFloorAngle _charactermovement 45.0)
  (Variables|/Script/Engine.CharacterMovementComponent|SetMaxStepHeight _charactermovement 45.0))

(fn ConstructionScript
  (|CallParentFunction))

(fn MatchDamageTraceData
  (params (DamageTraceName :type Name :default "None"))
  (bind _midtrace (Variables|Default|GetMidTrace))
  (bind _returnvalue (Transformation|GetWorldLocation _midtrace))
  (switch name DamageTraceName
    (:Default
      (Utilities|Debugging|RaiseScriptError "Invalid Damage Trace Provided!")
      (return "0, 0, 0" "0, 0, 0" 0.0))
    (:LeftHand
      (return (Transformation|GetWorldLocation (Variables|Default|GetLTraceStart)) (Transformation|GetWorldLocation (Variables|Default|GetLTraceEnd)) 4e+01))
    (:RightHand
      (return (Transformation|GetWorldLocation (Variables|Default|GetRTraceStart)) (Transformation|GetWorldLocation (Variables|Default|GetRTraceEnd)) 4e+01))
    (:Ball
      (return _returnvalue _returnvalue 1e+02))))