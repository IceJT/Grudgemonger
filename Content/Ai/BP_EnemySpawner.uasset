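; BP_EnemySpawner is a trigger volume that spawns a set of AI enemies the first time the player character overlaps its box.
; The construction script collects billboard components named with "Enemy_" as spawn points, matched by index to the classes in EnemyArray.
; Each spawned BP_Enemy receives a reference back to the spawner.
; When tracking is enabled, DecrementTotalEnemies counts kills and reports the total to the tracked event managers.
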(event OnComponentBeginOverlap(Box)
  (params (OverlappedComponent :type Primitive%20Component%20Object%20Reference) (OtherActor :type Actor%20Object%20Reference) (OtherComp :type Primitive%20Component%20Object%20Reference) (OtherBodyIndex :type Integer) (bFromSweep :type Boolean) (SweepResult :type Hit%20Result%20Structure%20%28by%20ref%29))
  ;[0.15 0.15 0.15 0.5] Character Overlap Spawn
  (if (== OtherActor (Variables|Default|GetAs%20BP%20Third%20Person%20Character))
    (Utilities|FlowControl|DoOnce false
      (:Completed
        (CallFunction|SpawnEnemies)))))

(event Custom|SpawnEnemies
  ;[0.15 0.15 0.15 0.5] Spawn Enemies
  (for (_array_element _array_index) (Variables|Default|GetEnemyArray)
    (bind _returnvalue (AI|SpawnAIFromClass _array_element 0 (Transformation|GetWorldLocation (Utilities|Array|Get(acopy) (Variables|Default|GetBillBoardArray) _array_index)) (Transformation|GetWorldRotation (Utilities|Array|Get(acopy) (Variables|Default|GetBillBoardArray) _array_index)) false 0))
    (bind _asbp_enemy (Utilities|Casting|CastToBP_Enemy _returnvalue))
    (Variables|/Game/Ai/BP_Enemy.BP_Enemy_C|SetSpawnerReference _asbp_enemy self)))

(event Custom|DecrementTotalEnemies
  ;[0.15 0.15 0.15 0.5] EventLogic
  (if (Variables|Default|GetTrackingEnemies?)
    (Variables|Default|SetEnemiesKilled (+ (Variables|Default|GetEnemiesKilled) 1))
    (for _array_element (Variables|Default|GetTrackedEventManagers)
      (Class|BPIEventLogic|EventCheck(Message) _array_element "None" (Variables|Default|GetEnemiesKilled) "NewEnumerator0"))))

(event EventBeginPlay
  ;[0.15 0.15 0.15 0.5] Set Initial Parameters
  (bind _asbp_third_person_character (Utilities|Casting|CastToBP_ThirdPersonCharacter (Game|GetPlayerCharacter 0)))
  (Variables|Default|SetAs%20BP%20Third%20Person%20Character _asbp_third_person_character)
  (Variables|Default|SetNumberOfInitialEnemies (Utilities|Array|Length (Variables|Default|GetEnemyArray)))
  (Variables|Default|SetEnemiesKilled 0))

(fn ConstructionScript
  (Utilities|Array|Clear (Variables|Default|GetBillBoardArray))
  (for _array_element (Actor|GetComponentsByClass "/Script/Engine.BillboardComponent")
    (if (Utilities|String|Contains (Utilities|GetDisplayName _array_element) "Enemy_")
      (Utilities|Array|Add (Variables|Default|GetBillBoardArray) _array_element))))