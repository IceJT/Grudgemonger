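; Enemy AI controller that starts the BT_Enemy behavior tree on BeginPlay and supplies its Blackboard with perception and state data.
; PawnSensing records a seen pawn as the target and a heard noise's location for investigation.
; Exposed events mirror grounded, stunned, dead and attacking states plus attack radius into Blackboard keys, leaving decisions to the tree.
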(event OnSeePawn(PawnSensing)
  (params (Pawn :type Pawn%20Object%20Reference))
  (AI|Components|Blackboard|SetValueasBool (Variables|Default|GetBlackboard) (Variables|Keys|GetBB_Bool_SeesTarget?) true)
  (AI|Components|Blackboard|SetValueasObject (Variables|Default|GetBlackboard) (Variables|Keys|GetBB_Object_TargetActor) Pawn))

(event OnHearNoise(PawnSensing)
  (params (Instigator :type Pawn%20Object%20Reference) (Location :type Vector%20%28by%20ref%29 :default "0, 0, 0") (Volume :type Float%20%28single-precision%29))
  (AI|Components|Blackboard|SetValueasBool (Variables|Default|GetBlackboard) (Variables|Keys|GetBB_Bool_InvestigatingSound?) true)
  (AI|Components|Blackboard|SetValueasVector (Variables|Default|GetBlackboard) (Variables|Keys|GetBB_Vector_LastHeardLocation) Location))

(event Custom|Die
  (AI|Components|Blackboard|SetValueasBool (Variables|Default|GetBlackboard) (Variables|Keys|GetBB_Bool_IsDead?) true))

(event Custom|UpdateMovementMode
  (params (OldMovementMode :type EMovementMode%20Enum :default "MOVE_None") (NewMovementMode :type EMovementMode%20Enum :default "MOVE_None"))
  (AI|Components|Blackboard|SetValueasBool (Variables|Default|GetBlackboard) (Variables|Keys|GetBB_Bool_IsGrounded?) (not (Utilities|Enum|Equal(Enum) NewMovementMode "MOVE_Falling"))))

(event Custom|UpdateIsStunned
  (params (New%20Value :type Boolean))
  (AI|Components|Blackboard|SetValueasBool (Variables|Default|GetBlackboard) (Variables|Keys|GetBB_Bool_IsStunned?) New%20Value))

(event Custom|IsAttacking?
  (params (IsAttacking :type Boolean))
  (AI|Components|Blackboard|SetValueasBool (Variables|Default|GetBlackboard) (Variables|Keys|GetBB_Bool_IsAttacking?) IsAttacking))

(event Custom|SetRadius
  (params (AttackRadius :type Float%20%28double-precision%29))
  (AI|Components|Blackboard|SetValueasFloat (Variables|Default|GetBlackboard) (Variables|Keys|GetBB_Float_AttackRadius) AttackRadius))

(event EventBeginPlay
  (AI|RunBehaviorTree "/Game/Ai/BT_Enemy.BT_Enemy"))

(fn ConstructionScript)