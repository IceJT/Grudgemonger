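; Player combat component for BP_ThirdPersonCharacter, handling target lock, melee combos, tap-to-dodge/hold-to-sprint and blocking.
; Attacks play data table montages by AttackType, with notifies cutting unqueued combos and motion-warping toward the enemy nearest the input or facing direction, within an angle threshold.
; A timer-looped sphere trace applies damage once per actor, with hitstop, camera shake, impact VFX and noise.
; Lock-on steers control rotation each tick.
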(event Custom|BeginDamageTrace
  (params (Damage :type Float%20%28double-precision%29) (DamageType :type Damage%20Type%20Class%20Reference) (DamageTraceName :type Name))
  ;[0.15 0.15 0.15 0.5] Sword Trace
  (Utilities|Array|Clear (Variables|Default|GetAlreadyDamagedActors))
  (bind _returnvalue (Utilities|Time|SetTimerbyEvent (delegate Custom|Damage%20Trace) 0.01 true))
  (Variables|/Script/Engine.CharacterMovementComponent|SetbAllowPhysicsRotationDuringAnimRootMotion (Variables|/Script/Engine.Character|GetCharacterMovement (Variables|Default|GetPlayer)) false))

(event Custom|Damage%20Trace
  (bind _player (Variables|Default|GetPlayer))
  (bind _player_2 (Variables|Default|GetPlayer))
  ;[0.15 0.15 0.15 0.5] Sword Trace
  (bind (_tracestart _traceend _tracesize) (Default|MatchDamageTraceData (Variables|Default|GetPlayer) (stale Custom|BeginDamageTrace DamageTraceName)))
  (bind (_outhit _returnvalue) (Collision|SphereTraceForObjects _tracestart _traceend _tracesize (Utilities|Array|MakeArray "ObjectTypeQuery3") false (Variables|Default|GetAlreadyDamagedActors) "None" true "(R=1.000000,G=0.000000,B=0.000000,A=1.000000)" "(R=0.000000,G=1.000000,B=0.000000,A=1.000000)" 1.0))
  (if _returnvalue
    (Game|Damage|ApplyDamage (.HitActor (Collision|BreakHitResult _outhit)) (* (Variables|Default|GetDamageMultiplier) (stale Custom|BeginDamageTrace Damage)) (Pawn|GetController _player_2) _player_2 (stale Custom|BeginDamageTrace DamageType)) ; If this was a custom function, we could only apply hitstun and sfx on confimration of a landed hit
    (Utilities|Array|Add (Variables|Default|GetAlreadyDamagedActors) (.HitActor (Collision|BreakHitResult _outhit)))
    (CallFunction|StartHitstop (Variables|Default|GetHitstopDuration))
    (Default|CameraShake (Variables|Default|GetPlayer))
    (Niagara|SpawnSystematLocation "/Game/FX/VFX/Vefects/Anime_VFX/Shared/Skills/NS_GenericImpact.NS_GenericImpact" (- (.ImpactPoint (Collision|BreakHitResult _outhit)) (* (.ImpactNormal (Collision|BreakHitResult _outhit)) 6e+01)) "0, 0, 0" "1.000000,1.000000,1.000000" true true "AutoRelease" false)
    (Class|PawnNoiseEmitterComponent|MakeNoise (Variables|/Game/Characters/ThirdPerson/Blueprints/BP_ThirdPersonCharacter.BP_ThirdPersonCharacter_C|GetPawnNoiseEmitter _player) _player 1.0 (- (.ImpactPoint (Collision|BreakHitResult _outhit)) (* (.ImpactNormal (Collision|BreakHitResult _outhit)) 6e+01)))))

(event Custom|End%20Damage%20Trace
  ;[0.15 0.15 0.15 0.5] Sword Trace
  (if (Utilities|Time|IsValidTimerHandle (stale Custom|BeginDamageTrace _returnvalue))
    (Utilities|Time|ClearandInvalidateTimerbyHandle (stale Custom|BeginDamageTrace _returnvalue))))

(event Custom|UpdateMotionWarpTarget
  (bind _player (Variables|Default|GetPlayer))
  ;[0.15 0.15 0.15 0.5] Motion Warping
  (bind (_foundtargetactor_ _warptarget) (CallFunction|GetClosestMotionWarpTarget))
  (if (and _foundtargetactor_ (not (AI|Components|NavMovement|IsFalling (Variables|/Script/Engine.Character|GetCharacterMovement (Variables|Default|GetPlayer)))))
    (if (< (Variables|Default|GetMotionWarpFaceThreshold) (Math|Vector|DotProduct (Math|Rotator|GetRotationXVector (Transformation|GetActorRotation _player)) (Math|Rotator|GetRotationXVector (Math|Rotator|FindLookatRotation (Transformation|GetActorLocation _player) (Transformation|GetActorLocation _warptarget))))) ; Is our target close enough to our rotation to justify snapping to?
      (Class|MotionWarpingComponent|AddorUpdateWarpTarget (Variables|/Game/Characters/ThirdPerson/Blueprints/BP_ThirdPersonCharacter.BP_ThirdPersonCharacter_C|GetMotionWarping (Variables|Default|GetPlayer)) (Utilities|Struct|MakeMotionWarpingTarget "Target" (Transformation|GetActorLocation _warptarget) (Math|Rotator|MakeRotfromX (Math|Rotator|GetRotationXVector (Math|Rotator|FindLookatRotation (Transformation|GetActorLocation _player) (Transformation|GetActorLocation _warptarget)))) 0 "None" false "TargetsForwardVector" "0.000000,0.000000,0.000000" "0.000000,0.000000,0.000000" 0))
      (else
        (Class|MotionWarpingComponent|RemoveWarpTarget (Variables|/Game/Characters/ThirdPerson/Blueprints/BP_ThirdPersonCharacter.BP_ThirdPersonCharacter_C|GetMotionWarping (Variables|Default|GetPlayer)) "Target" :!label _label)))
    (else
      (goto _label))))

(event Custom|SetViewModel
  (params (Viewmodel :type View%20Model%20Stats%20Player%20Object%20Reference))
  ;[0.15 0.15 0.15 0.5] Set Viewmodel
  (Variables|Default|SetViewmodel Viewmodel))

(event Custom|StartHitstop
  (params (Duration :type Float%20%28double-precision%29))
  (bind _player (Variables|Default|GetPlayer))
  (bind _mesh (Variables|/Script/Engine.Character|GetMesh _player))
  ;[0.15 0.15 0.15 0.5] Hitstop
  (Variables|/Script/Engine.SkeletalMeshComponent|SetbPauseAnims _mesh true)
  (Utilities|FlowControl|RetriggerableDelay Duration)
  (Variables|/Script/Engine.SkeletalMeshComponent|SetbPauseAnims _mesh false))

(event Custom|ResetSprintEvent
  (bind _player (Variables|Default|GetPlayer))
  ;[0.15 0.15 0.15 0.5] Dodge
  (Utilities|FlowControl|DoOnce false) ; enters at Reset
)

(event Custom|StopBlocking
  (bind _player (Variables|Default|GetPlayer))
  ;[0.15 0.15 0.15 0.5] Blocking
  (Variables|Default|SetIsBlocking? false)
  (Character|UnCrouch _player)
  (Development|SetHiddeninGame (Variables|/Game/Characters/ThirdPerson/Blueprints/BP_ThirdPersonCharacter.BP_ThirdPersonCharacter_C|GetSM_Cane _player) false false)
  (Rendering|Material|SetScalarParameterValue "/Game/Characters/_Commons/Materials/MPC_GlobalCharacterEffects.MPC_GlobalCharacterEffects" "VignetteBlend" 0.0 :!class /Script/Engine.KismetMaterialLibrary))

(event Input|EnhancedActionEvents|EnhancedInputActionIA_Lock
  (params (ActionValue :type Boolean) (ElapsedSeconds :type Float%20%28double-precision%29) (TriggeredSeconds :type Float%20%28double-precision%29) (InputAction :type Input%20Action%20Object%20Reference :default "/Game/Characters/ThirdPerson/Input/Actions/IA_Lock.IA_Lock"))
  (bind _returnvalue (Game|GetPlayerCameraManager 0))
  (bind _player (Variables|Default|GetPlayer))
  (bind _player_2 (Variables|Default|GetPlayer))
  (bind _transformcomponent (Variables|/Script/Engine.PlayerCameraManager|GetTransformComponent _returnvalue))
  (bind _charactermovement (Variables|/Script/Engine.Character|GetCharacterMovement _player))
  (bind _charactermovement_2 (Variables|/Script/Engine.Character|GetCharacterMovement _player_2))
  (bind _returnvalue_2 (Transformation|GetWorldLocation _transformcomponent))
  ;[0.15 0.15 0.15 0.5] TargetLock
  (:Started
    (Variables|Default|GetTargetLockActor
      (:then
        (bind _asbp_enemy (Utilities|Casting|CastToBP_Enemy (Variables|Default|GetTargetLockActor)))
        (Default|DisableWidget _asbp_enemy)
        (Variables|Default|SetTargetLockActor 0)
        (Variables|/Script/Engine.CharacterMovementComponent|SetbOrientRotationToMovement _charactermovement true)
        (Variables|/Script/Engine.CharacterMovementComponent|SetbUseControllerDesiredRotation _charactermovement false)
        (bind _viewmodel (Variables|Default|GetViewmodel)
          (:then
            (Variables|/Game/UI/ViewModelStatsParent.ViewModelStatsParent_C|SetLockedOn? _viewmodel false))
          (:else)))
      (:else
        (bind (_outhit _returnvalue_3) (Collision|SphereTraceForObjects (Transformation|GetWorldLocation (Variables|/Script/Engine.Actor|GetRootComponent (Variables|Default|GetPlayer))) (+ (Math|Vector|MakeVector (.x _returnvalue_2) (.y _returnvalue_2) (+ (.z _returnvalue_2) 2e+01)) (* (Math|Vector|GetForwardVector (Transformation|GetWorldRotation _transformcomponent)) 4e+03)) 1.5e+02 (Utilities|Array|MakeArray "ObjectTypeQuery3") false 0 "None"))
        (if _returnvalue_3
          (bind _asbp_enemy_2 (Utilities|Casting|CastToBP_Enemy (.HitActor (Collision|BreakHitResult _outhit))))
          (if (not (Variables|/Game/Ai/BP_Enemy.BP_Enemy_C|GetIsDead? _asbp_enemy_2))
            (Variables|Default|SetTargetLockActor (.HitActor (Collision|BreakHitResult _outhit)))
            (Variables|/Script/Engine.CharacterMovementComponent|SetbOrientRotationToMovement _charactermovement_2 false)
            (Variables|/Script/Engine.CharacterMovementComponent|SetbUseControllerDesiredRotation _charactermovement_2 true)
            (bind _asbp_enemy_3 (Utilities|Casting|CastToBP_Enemy (Variables|Default|GetTargetLockActor)))
            (Default|EnableWidget _asbp_enemy_3)
            (bind _viewmodel_2 (Variables|Default|GetViewmodel)
              (:then
                (Variables|/Game/UI/ViewModelStatsParent.ViewModelStatsParent_C|SetLockedOn? _viewmodel_2 true))
              (:else))))))))

(event Input|EnhancedActionEvents|EnhancedInputActionIA_Attack
  (params (ActionValue :type Boolean) (ElapsedSeconds :type Float%20%28double-precision%29) (TriggeredSeconds :type Float%20%28double-precision%29) (InputAction :type Input%20Action%20Object%20Reference :default "/Game/Characters/ThirdPerson/Input/Actions/IA_Attack.IA_Attack"))
  ;[0.15 0.15 0.15 0.5] Attack
  (:Started
    (Variables|Default|SetCanSprint? false)
    (bind _returnvalue (Utilities|GetDataTableRow (Variables|Default|GetAttacksData) (Utilities|String|StringToName (Utilities|String|EnumtoString (Variables|/Game/Characters/ThirdPerson/Blueprints/BP_ThirdPersonCharacter.BP_ThirdPersonCharacter_C|GetAttackType (Variables|Default|GetPlayer)))))
      (:then
        (Variables|Default|SetAttackAnimation (Utilities|Struct|BreakS_AttackProperties _returnvalue))
        (if (not (Variables|Default|GetIsAttacking?))
          (Variables|Default|SetIsAttacking? true)
          (bind _notifyname (Animation|Montage|PlayMontage (Variables|/Script/Engine.Character|GetMesh (Variables|Default|GetPlayer)) (Variables|Default|GetAttackAnimation))
            (:then
              (Default|IncreaseValue (Variables|/Game/Characters/ThirdPerson/Blueprints/BP_ThirdPersonCharacter.BP_ThirdPersonCharacter_C|GetBP_Stats (Variables|Default|GetPlayer)) "NewEnumerator1" (Variables|Default|GetAttackStaminaDrain) :!label _label))
            (:OnCompleted
              (Variables|Default|SetIsAttacking? false :!label _label_2)
              (Variables|Default|SetCombo? false)
              (Variables|Default|SetCanSprint? true))
            (:OnInterrupted
              (goto _label_2))
            (:OnNotifyBegin
              (switch name _notifyname
                (:ComboCutoff
                  (if (and (Variables|Default|GetIsAttacking?) (Variables|Default|GetCombo?))
                    (Variables|Default|SetCombo? false)
                    (goto _label)
                    (else
                      (Animation|Montage|MontageStop (Components|SkeletalMesh|GetAnimInstance (Variables|/Script/Engine.Character|GetMesh (Variables|Default|GetPlayer))) 0.2 0))))
                (:UpdateWarpTarget
                  (CallFunction|UpdateMotionWarpTarget)))))
          (else
            (Variables|Default|SetCombo? true))))
      (:RowNotFound
        (Development|PrintString "Hello")))))

(event Input|EnhancedActionEvents|EnhancedInputActionIA_Dodge
  (params (ActionValue :type Boolean) (ElapsedSeconds :type Float%20%28double-precision%29) (TriggeredSeconds :type Float%20%28double-precision%29) (InputAction :type Input%20Action%20Object%20Reference :default "/Game/Characters/ThirdPerson/Input/Actions/IA_Dodge.IA_Dodge"))
  (bind _player (Variables|Default|GetPlayer))
  (bind _player_2 (Variables|Default|GetPlayer))
  ;[0.15 0.15 0.15 0.5] Dodge
  (:Triggered
    (if (Variables|Default|GetCanSprint?)
      (if (>= TriggeredSeconds 0.31)
        (Utilities|FlowControl|DoOnce false
          (:Completed
            (Animation|Montage|PlayMontage (Variables|/Script/Engine.Character|GetMesh (Variables|Default|GetPlayer)) "/Game/Characters/Sigurd/Animations/AS_Sigurd_Sprint_Start_Montage.AS_Sigurd_Sprint_Start_Montage"
              (:then
                (Default|StartSprinting _player_2)
                (Variables|/Game/Characters/ThirdPerson/Blueprints/BP_ThirdPersonCharacter.BP_ThirdPersonCharacter_C|SetAttackType _player_2 "NewEnumerator2")
                (CallFunction|StopBlocking))))))))
  (:Completed
    (CallFunction|ResetSprintEvent)
    (if (Variables|/Game/Characters/ThirdPerson/Blueprints/BP_ThirdPersonCharacter.BP_ThirdPersonCharacter_C|GetSprinting? (Variables|Default|GetPlayer))
      (Animation|Montage|PlayMontage (Variables|/Script/Engine.Character|GetMesh (Variables|Default|GetPlayer)) "/Game/Characters/Sigurd/Animations/AS_Sigurd_Sprint_End_Montage.AS_Sigurd_Sprint_End_Montage"
        (:then
          _)))
    (Default|ResetMovement (Variables|Default|GetPlayer))
    (Variables|/Game/Characters/ThirdPerson/Blueprints/BP_ThirdPersonCharacter.BP_ThirdPersonCharacter_C|SetAttackType (Variables|Default|GetPlayer) "NewEnumerator0")
    (if (<= TriggeredSeconds 0.3)
      (if (not (Variables|Default|GetIsDodging?))
        (Variables|Default|SetIsDodging? true)
        (Utilities|FlowControl|Sequence
          (:then_0
            (Variables|Default|SetMovementDirection "NewEnumerator0"))
          (:then_1
            (Animation|Montage|PlayMontage (Variables|/Script/Engine.Character|GetMesh (Variables|Default|GetPlayer)) (Utilities|Select :Index (Variables|Default|GetMovementDirection) :NewEnumerator0 "/Game/Characters/Sigurd/Prototype/Anims/Dodge_F_Montage.Dodge_F_Montage" :NewEnumerator1 "/Game/Characters/Sigurd/Prototype/Anims/Dodge_L_Montage.Dodge_L_Montage" :NewEnumerator2 "/Game/Characters/Sigurd/Prototype/Anims/Dodge_B_Montage.Dodge_B_Montage" :NewEnumerator3 "/Game/Characters/Sigurd/Prototype/Anims/Dodge_R_Montage.Dodge_R_Montage")
              (:then
                (Default|IncreaseValue (Variables|/Game/Characters/ThirdPerson/Blueprints/BP_ThirdPersonCharacter.BP_ThirdPersonCharacter_C|GetBP_Stats (Variables|Default|GetPlayer)) "NewEnumerator1" -25.0)
                (Character|LaunchCharacter _player (* (Math|Vector|GetForwardVector (Variables|/Script/Engine.Character|GetCapsuleComponent _player)) "1500.000000,1500.000000,0.000000") false false))
              (:OnCompleted
                (Variables|Default|SetIsDodging? false :!label _label))
              (:OnInterrupted
                (goto _label)))))))))

(event Input|EnhancedActionEvents|EnhancedInputActionIA_Block
  (params (ActionValue :type Boolean) (ElapsedSeconds :type Float%20%28double-precision%29) (TriggeredSeconds :type Float%20%28double-precision%29) (InputAction :type Input%20Action%20Object%20Reference :default "/Game/Characters/ThirdPerson/Input/Actions/IA_Block.IA_Block"))
  (bind _player (Variables|Default|GetPlayer))
  (bind _player_2 (Variables|Default|GetPlayer))
  (bind _mesh (Variables|/Script/Engine.Character|GetMesh _player))
  (bind _sm_cane (Variables|/Game/Characters/ThirdPerson/Blueprints/BP_ThirdPersonCharacter.BP_ThirdPersonCharacter_C|GetSM_Cane _player_2))
  (bind _returnvalue (Components|SkeletalMesh|GetAnimInstance _mesh))
  ;[0.15 0.15 0.15 0.5] Blocking
  (:Started
    (if (not (AI|Components|NavMovement|IsFalling (Variables|/Script/Engine.Character|GetCharacterMovement (Variables|Default|GetPlayer))))
      (Variables|Default|SetIsBlocking? true)
      (Variables|/Game/Characters/ThirdPerson/Blueprints/BP_ThirdPersonCharacter.BP_ThirdPersonCharacter_C|SetAttackType _player_2 "NewEnumerator0")
      (Character|Crouch _player_2)
      (Development|SetHiddeninGame _sm_cane true false)
      (Rendering|Material|SetScalarParameterValue "/Game/Characters/_Commons/Materials/MPC_GlobalCharacterEffects.MPC_GlobalCharacterEffects" "VignetteBlend" 1.0 :!class /Script/Engine.KismetMaterialLibrary)
      (Animation|Montage|MontageStop _returnvalue 0.0 (Animation|Montage|GetCurrentActiveMontage _returnvalue))))
  (:Completed
    (Variables|Default|SetIsBlocking? false)
    (Character|UnCrouch _player_2)
    (Development|SetHiddeninGame _sm_cane false false)
    (Rendering|Material|SetScalarParameterValue "/Game/Characters/_Commons/Materials/MPC_GlobalCharacterEffects.MPC_GlobalCharacterEffects" "VignetteBlend" 0.0 :!class /Script/Engine.KismetMaterialLibrary)))

(event EventTick
  (params (DeltaSeconds :type Float%20%28single-precision%29))
  (bind _player (Variables|Default|GetPlayer))
  (bind _targetlockactor (Variables|Default|GetTargetLockActor))
  (bind _returnvalue (Transformation|GetActorLocation _player))
  (bind _returnvalue_2 (Transformation|GetActorLocation _targetlockactor))
  (bind _returnvalue_3 (Math|Rotator|FindLookatRotation _returnvalue _returnvalue_2))
  ;[0.15 0.15 0.15 0.5] Lock On Focus
  (Variables|Default|GetTargetLockActor
    (:then
      (Pawn|SetControlRotation (Pawn|GetController (Variables|Default|GetPlayer)) (Math|Rotator|MakeRotator (.roll _returnvalue_3) (+ (.pitch _returnvalue_3) -2e+01) (.yaw _returnvalue_3))))
    (:else)))

(event EventBeginPlay
  ;[0.15 0.15 0.15 0.5] Set Player Reference
  (bind _asbp_third_person_character (Utilities|Casting|CastToBP_ThirdPersonCharacter (Components|GetOwner)))
  (Variables|Default|SetPlayer _asbp_third_person_character))

(event Input|KeyboardEvents|DebugKeyT
  (params (Key :type Key%20Structure) (ActionValue :type Input%20Action%20Value%20Structure))
  ;[0.15 0.15 0.15 0.5] Attack
  (:Pressed
    (Animation|Montage|PlayMontage (Variables|/Script/Engine.Character|GetMesh (Variables|Default|GetPlayer)) "/Game/Characters/Sigurd/Animations/SwordAttackCombo_Montage.SwordAttackCombo_Montage")))

(fn GetClosestMotionWarpTarget
  (bind _player (Variables|Default|GetPlayer))
  (bind _player_2 (Variables|Default|GetPlayer))
  (if (Variables|/Script/Engine.CharacterMovementComponent|GetbAllowPhysicsRotationDuringAnimRootMotion (Variables|/Script/Engine.Character|GetCharacterMovement (Variables|Default|GetPlayer)))
    ;[0.15 0.15 0.15 0.5] Set a target location in front of the player input, this will be used to check which enemy is closest to our desired attack direction
    (LocalVariables|SetDesiredTargetLocation (+ (Transformation|GetActorLocation _player_2) (* 1.5e+02 (Math|Vector|GetForwardVector (Math|Conversions|RotationFromXVector (Class|Pawn|GetLastMovementInputVector _player_2))))))
    (else
      ;[0.15 0.15 0.15 0.5] Set a target location in front of sigurd instead of input direction if root motion input is disabled
      (LocalVariables|SetDesiredTargetLocation (+ (Transformation|GetActorLocation _player) (* 1.5e+02 (Transformation|GetActorForwardVector _player))))))
  ;[0.15 0.15 0.15 0.5] Loop through each actor in our motion warp sphere collision area
  (for (_array_element _array_index) (Collision|GetOverlappingActors (Variables|/Game/Characters/ThirdPerson/Blueprints/BP_ThirdPersonCharacter.BP_ThirdPersonCharacter_C|GetMotionWarpRadius (Variables|Default|GetPlayer)) "/Game/Ai/BP_Enemy.BP_Enemy_C" :!class /Script/Engine.PrimitiveComponent)
    ;[0.15 0.15 0.15 0.5] If this is the initial actor OR this actor is closer than the last, Update new closest actor
    (if (or (== _array_index 0) (< (Math|Vector|Distance(Vector) (Transformation|GetActorLocation _array_element) (LocalVariables|GetDesiredTargetLocation)) (LocalVariables|GetClosestActorDistance)))
      (LocalVariables|SetClosestActorDistance (Math|Vector|Distance(Vector) (Transformation|GetActorLocation _array_element) (LocalVariables|GetDesiredTargetLocation)))
      (LocalVariables|SetClosestActor _array_element)))
  ;[0.15 0.15 0.15 0.5] Finish loop and return Found if an actor was fetched, else return not Found
  (Utilities|IsValid (LocalVariables|GetClosestActor)
    (:Is%20Valid
      (return true (LocalVariables|GetClosestActor)))
    (:Is%20Not%20Valid
      (return false 0))))