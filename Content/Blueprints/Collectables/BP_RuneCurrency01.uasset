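; BP_RuneCurrency01 is a collectable rune currency actor that shows a randomly chosen rune mesh.
; On BeginPlay it calls the parent logic, then ChooseMesh sets the static mesh to a random entry from the Runes array, guarded by a DoOnce.
; It adds no overlap, tick or construction behavior of its own.
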(event Custom|Choose%20Mesh
  (bind _runes (Variables|Default|GetRunes))
  ;[0.15 0.15 0.15 0.5] Setting Mesh to be one of the random runes
  (Utilities|FlowControl|DoOnce false
    (:Completed
      (Components|StaticMesh|SetStaticMesh (Variables|Default|GetStaticMesh) (Utilities|Array|Get(acopy) _runes (Math|Random|RandomIntegerinRange 0 (- (Utilities|Array|Length _runes) 1)))))))

(event EventBeginPlay
  (|CallParentFunction)
  (CallFunction|ChooseMesh))

(event Collision|EventActorBeginOverlap
  (params (OtherActor :type Actor%20Object%20Reference)))

(event EventTick
  (params (DeltaSeconds :type Float%20%28single-precision%29))
  (|CallParentFunction DeltaSeconds) ; This node is disabled and will not be called.\nDrag off pins to build functionality.
)

(fn ConstructionScript
  (|CallParentFunction))