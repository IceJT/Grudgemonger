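; Collectable pickup that reacts once to overlap by the third-person character, hiding its mesh, switching Niagara effects and playing a rune collect sound.
; A 0.3-second timer from BeginPlay clears DelayCollect, the flag that gates collection.
; MoveTo uses a timeline to move the actor between two given locations, with separate curves for travel, height offset and mesh scale.
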(event OnComponentBeginOverlap(Sphere)
  (params (OverlappedComponent :type Primitive%20Component%20Object%20Reference) (OtherActor :type Actor%20Object%20Reference) (OtherComp :type Primitive%20Component%20Object%20Reference) (OtherBodyIndex :type Integer) (bFromSweep :type Boolean) (SweepResult :type Hit%20Result%20Structure%20%28by%20ref%29))
  (Class|KismetSystemLibrary|IsObjectOfSoftClass OtherActor "/Game/Characters/ThirdPerson/Blueprints/BP_ThirdPersonCharacter.BP_ThirdPersonCharacter_C"
    (:True
      (if (not (Variables|Default|GetDelayCollect?))
        (Utilities|FlowControl|DoOnce false
          (:Completed
            (Development|SetHiddeninGame (Variables|Default|GetStaticMesh) true true)
            (Components|Activation|Deactivate (Variables|Default|GetNiagara))
            (Components|Activation|Activate (Variables|Default|GetNiagara1) true)
            (Audio|PlaySound2D "/Game/Sound/SFX/Collectibles/SFX_Collect_Rune.SFX_Collect_Rune" 1.0 1.0 0.0 0 0)))))))

(event Custom|MoveTo
  (params (StartingLocation :type Vector) (TargetLocation :type Vector))
  (bind (_direction _lerp _height _scale) (Timeline|Timeline PlayFromStart)
    (:Update
      (Transformation|SetActorLocation (Math|Vector|Lerp(Vector) (Math|Vector|Lerp(Vector) StartingLocation (+ TargetLocation "0.000000,0.000000,20.000000") _lerp) (+ (Math|Vector|Lerp(Vector) StartingLocation (+ TargetLocation "0.000000,0.000000,20.000000") _lerp) "0.000000,0.000000,200.000000") _height) false false)
      (Transformation|SetRelativeScale3D (Variables|Default|GetStaticMesh) (Math|Conversions|ToVector(Float) (Math|Float|Lerp 0.0 2.0 _scale))))))

(event EventBeginPlay
  (Utilities|Time|SetTimerbyFunctionName 0 "BarCollectionForATime" 0.3))

(event EventTick
  (params (DeltaSeconds :type Float%20%28single-precision%29)))

(fn ConstructionScript)

(fn BarCollectionforATime
  (Variables|Default|SetDelayCollect? false))