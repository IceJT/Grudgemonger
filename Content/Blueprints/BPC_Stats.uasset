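; BPC_Stats is an actor component that tracks health and stamina and sends DieMessage to its owner when health runs out.
; IncreaseValue applies clamped changes to either stat and pushes results into a Viewmodel for the UI.
; A fast looping timer regenerates stamina.
; Stamina drains restart a cooldown timer that pauses regeneration, but only while the Viewmodel is valid.
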(event Custom|Die
  (Class|BPIDamage|Die(Message) (Components|GetOwner)))

(event Custom|SetHealthProgressBar
  (params (HealthProgressBar :type Progress%20Bar%20Object%20Reference))
  (Variables|Default|SetHealth%20Progress%20Bar HealthProgressBar))

(event Custom|SetStaminaProgressBar
  (params (StaminaProgressBar :type Progress%20Bar%20Object%20Reference))
  (Variables|Default|SetStaminaProgressBar StaminaProgressBar))

(event Custom|RegainStamina
  (if (Variables|Default|GetRegainStamina?)
    (CallFunction|IncreaseValue "NewEnumerator1" 0.35)))

(event Custom|SetViewModel
  (params (Viewmodel :type View%20Model%20Stats%20Parent%20Object%20Reference))
  (Variables|Default|SetViewmodel Viewmodel))

(event Custom|StartStaminaCooldown
  (Variables|Default|SetRegainStamina? false)
  (if (Utilities|Time|IsTimerActivebyHandle (stale _returnvalue))
    (Utilities|Time|ClearandInvalidateTimerbyHandle (stale _returnvalue)))
  (bind _returnvalue (Utilities|Time|SetTimerbyEvent (delegate Custom|FinishStaminaCooldown) 2.0)))

(event Custom|FinishStaminaCooldown
  (Variables|Default|SetRegainStamina? true))

(event EventBeginPlay
  (Utilities|Time|SetTimerbyEvent (delegate Custom|RegainStamina) 0.01 true)
  (bind _viewmodel (Variables|Default|GetViewmodel)
    (:then
      (Variables|/Game/UI/ViewModelStatsParent.ViewModelStatsParent_C|SetHealthCurrent _viewmodel (Variables|Default|GetHealth)))
    (:else)))

(fn IncreaseValue
  (params (Stat :type E_Stats%20Enum :default "NewEnumerator0") (Float :type Float%20%28double-precision%29))
  (Variables|Default|SetFloatValue Float)
  (switch Utilities|FlowControl|Switch|SwitchonE_Stats Stat
    (:NewEnumerator0
      ;[0.15 0.15 0.15 0.5] Health
      (if (> (Math|Float|Absolute(Float) (Variables|Default|GetFloatValue)) 0.1)
        (Variables|Default|SetHealth (Math|Float|Clamp(Float) (+ (Variables|Default|GetHealth) (Variables|Default|GetFloatValue)) 0.0 (Variables|Default|GetMaxHealth)))
        (Utilities|FlowControl|Sequence
          (:then_0
            (if (<= (Variables|Default|GetHealth) 0.0)
              (CallFunction|Die)))
          (:then_1
            (bind _viewmodel (Variables|Default|GetViewmodel)
              (:then
                (Variables|/Game/UI/ViewModelStatsParent.ViewModelStatsParent_C|SetHealthCurrent _viewmodel (Variables|Default|GetHealth)))
              (:else))))))
    (:NewEnumerator1
      ;[0.15 0.15 0.15 0.5] Stamina
      (Variables|Default|SetStamina (Math|Float|Clamp(Float) (+ (Variables|Default|GetStamina) (Variables|Default|GetFloatValue)) 0.0 (Variables|Default|GetMaxStamina)))
      (bind _viewmodel_2 (Variables|Default|GetViewmodel)
        (:then
          (if (>= (/ (Variables|Default|GetStamina) (Variables|Default|GetMaxStamina)) 1e+02)
            (Utilities|FlowControl|DoOnce false
              (:Completed
                _)))
          (Variables|/Game/UI/ViewModelStatsParent.ViewModelStatsParent_C|SetStamina _viewmodel_2 (/ (Variables|Default|GetStamina) (Variables|Default|GetMaxStamina)))
          (if (< (Variables|Default|GetFloatValue) 0.0)
            (CallFunction|StartStaminaCooldown)))
        (:else)))))