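; BP_LivingCharacter is a character Blueprint that holds health and stamina, with getters for current values and percentages of maximum.
; ApplyHealth adds a delta, clamps it between the minimum and maximum, then calls OnHealthChange.
; ApplyStamina follows the same pattern and calls OnStaminaChanged, but writes its result to CurrentHealth and caps it at zero instead of StaminaMax.
; BeginPlay and both change events are empty here.
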(event Custom|OnStaminaChanged)

(event Custom|OnHealthChange)

(event EventBeginPlay)

(fn ConstructionScript)

(fn ApplyHealth
  (params (Value :type Float%20%28double-precision%29))
  (bind _output_get (Variables|Attributes|SetCurrentHealth (Math|Float|Min(Float) (Math|Float|Max(Float) (+ Value (Variables|Attributes|GetCurrentHealth)) (Variables|Attributes|GetMinHealth)) (Variables|Attributes|GetMaxHealth))))
  (CallFunction|OnHealthChange)
  (return _output_get))

(fn GetCurrentHealth
  (return (Variables|Attributes|GetCurrentHealth)))

(fn GetCurrentHealthPercentage
  (return (Math|Float|SafeDivide (Variables|Attributes|GetCurrentHealth) (Variables|Attributes|GetMaxHealth))))

(fn GetCurrentStamina
  (return (Variables|Attributes|GetStaminaCurrent)))

(fn GetCurrentStaminaPercentage
  (return (Math|Float|SafeDivide (Variables|Attributes|GetStaminaCurrent) (Variables|Attributes|GetStaminaMax))))

(fn ApplyStamina
  (params (Value :type Float%20%28double-precision%29))
  (bind _output_get (Variables|Attributes|SetCurrentHealth (Math|Float|Min(Float) (Math|Float|Max(Float) (+ Value (Variables|Attributes|GetStaminaCurrent)) (Variables|Attributes|GetStaminaMin)) 0.0)))
  (CallFunction|OnStaminaChanged)
  (return _output_get))